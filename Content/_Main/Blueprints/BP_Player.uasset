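; BP_Player is the player pawn, with jump and left/right movement driven by Enhanced Input.
; On BeginPlay it adds the input mapping context, switches to game-only input, creates the W_HUD widget and caches the GM_MasterMode game mode.
; Damage reduces MaxHealth directly, as it doubles as current health, and updates the HUD.
; At zero health it flags the player dead and notifies the game mode.
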(event `self.ReceiveBeginPlay`
  ;[0 0 1] BeginPlay
  (bind _asplayer_controller (cast `PlayerController` (`self.GetController`)))
  (`/Engine/EditorBlueprintResources/StandardMacros.IsValid` _asplayer_controller
    (:`Is Valid`
      (`EnhancedInputSubsystemInterface.AddMappingContext` (pcsubsystem `EnhancedInputLocalPlayerSubsystem` _asplayer_controller) "/Game/_Main/Inputs/IMC_PlayerInput.IMC_PlayerInput" 0 (struct))
      (`self.Initialize`))))

(event `EnhancedInput|/Game/_Main/Inputs/InputActions/IA_Jump`
  (params (ActionValue :type Boolean) (ElapsedSeconds :type "Float (double-precision)") (TriggeredSeconds :type "Float (double-precision)") (InputAction :type "InputAction Object Reference" :default "/Game/_Main/Inputs/InputActions/IA_Jump.IA_Jump"))
  ;[1 0 1] Player Jump Control
  (:`Started`
    (`self.Jump`))
  (:`Completed`
    (`self.StopJumping`)))

(event `EnhancedInput|/Game/_Main/Inputs/InputActions/IA_MoveRight`
  (params (ActionValue :type "Vector2D Structure") (ElapsedSeconds :type "Float (double-precision)") (TriggeredSeconds :type "Float (double-precision)") (InputAction :type "InputAction Object Reference" :default "/Game/_Main/Inputs/InputActions/IA_MoveRight.IA_MoveRight"))
  ;[1 0 1] Player Movement Left/Right
  (:`Triggered`
    (`self.AddMovementInput` (`KismetMathLibrary.Conv_Vector2DToVector` ActionValue))))

(event `EnhancedInput|/Game/_Main/Inputs/InputActions/IA_MoveLeft`
  (params (ActionValue :type "Vector2D Structure") (ElapsedSeconds :type "Float (double-precision)") (TriggeredSeconds :type "Float (double-precision)") (InputAction :type "InputAction Object Reference" :default "/Game/_Main/Inputs/InputActions/IA_MoveLeft.IA_MoveLeft"))
  ;[1 0 1] Player Movement Left/Right
  (:`Triggered`
    (`self.AddMovementInput` (* (`KismetMathLibrary.Conv_Vector2DToVector` ActionValue) (-1.0 0.0 0.0)))))

(event `self.ReceiveAnyDamage`
  (params (Damage :type "Float (single-precision)") (DamageType :type "DamageType Object Reference") (InstigatedBy :type "Controller Object Reference") (DamageCauser :type "Actor Object Reference"))
  (if (not (`self.IsDead?`))
    (bind _output_get (set `self.MaxHealth` (`KismetMathLibrary.FClamp` (- (`self.MaxHealth`) Damage) 0.0 (`self.MaxHealth`))))
    (`/Game/_Main/Blueprints/UMG/W_HUD.RemoveHealth` (`self.HUDWidget_REF`) _output_get)
    (if (<= (`self.MaxHealth`) 0.0)
      (set `self.IsDead?` true)
      (`/Game/_Main/Blueprints/GameModes/GM_MasterMode.PlayerDeath` (`self.GM_REF`)))))

(fn `Initialize`
  (bind _returnvalue (`GameplayStatics.GetPlayerController` 0))
  (`self.EnableInput` _returnvalue)
  (set `PlayerController.bShowMouseCursor` false _returnvalue)
  (`WidgetBlueprintLibrary.SetInputMode_GameOnly` _returnvalue)
  (bind _returnvalue_2 (`|CreateWidget` "/Game/_Main/Blueprints/UMG/W_HUD.W_HUD_C"))
  (bind _output_get (set `self.HUDWidget_REF` _returnvalue_2))
  (`UserWidget.AddToViewport` _output_get 0)
  (bind _asgm_stick_it_out (cast `/Game/_Main/Blueprints/GameModes/GM_MasterMode` (`GameplayStatics.GetGameMode`)))
  (set `self.GM_REF` _asgm_stick_it_out))

(fn `UserConstructionScript`)