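; Base game mode that handles player death for a sprite-based BP_Player character.
; On BeginPlay it caches a reference to the player character.
; PlayerDeath hides the player's sprite, sets global time dilation to zero, switches to cursor-driven UI-only input, then immediately opens the level named by LevelName.
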(event `self.ReceiveBeginPlay`
  (bind _asbp_player (cast `/Game/_Main/Blueprints/BP_Player` (`GameplayStatics.GetPlayerCharacter` 0)))
  (set `self.Player_REF` _asbp_player))

(fn `PlayerDeath`
  (bind _returnvalue (`GameplayStatics.GetPlayerController` 0))
  (`SceneComponent.SetVisibility` (`/Game/_Main/Blueprints/BP_Player.PaperSprite` (`self.Player_REF`)) false false)
  (`GameplayStatics.SetGlobalTimeDilation` 0.0)
  (set `PlayerController.bShowMouseCursor` true _returnvalue)
  (`WidgetBlueprintLibrary.SetInputMode_UIOnlyEx` _returnvalue null)
  (`GameplayStatics.OpenLevel` (`self.Level Name`)))

(fn `UserConstructionScript`)