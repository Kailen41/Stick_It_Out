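; BP_SpikeTrap is an obstacle actor that moves spikes vertically and sends the player to the 02_Obstacles level on contact.
; On BeginPlay, a timeline starts at a configurable play rate and lerps the movement component's relative Z location between two fixed heights.
; A box collider overlap with any valid actor tagged Player opens that level by name.
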(event `self.ReceiveBeginPlay`
  (`TimelineComponent.SetPlayRate` (`self.TrapMovement_TL`) (`self.PlayRate`))
  (`self.SpikeTrap`))

(event `SpikeTrap`
  (bind (_direction _alpha_movement) (`Timeline|TrapMovement_TL` :`NewTime` (`self.PlayRate`))
    (:`Update`
      (`SceneComponent.K2_SetRelativeLocation` (`self.MovementCompoent`) (`KismetMathLibrary.MakeVector` 0.0 0.0 (`KismetMathLibrary.Lerp` 0.0 300.0 _alpha_movement)) false false))))

(event `self.Box Collider.OnComponentBeginOverlap`
  (params (OverlappedComponent :type "PrimitiveComponent Object Reference") (OtherActor :type "Actor Object Reference") (OtherComp :type "PrimitiveComponent Object Reference") (OtherBodyIndex :type Integer) (bFromSweep :type Boolean) (SweepResult :type "HitResult Structure (by ref)"))
  (`/Engine/EditorBlueprintResources/StandardMacros.IsValid` OtherActor
    (:`Is Valid`
      (if (`self.ActorHasTag` OtherActor "Player")
        (`GameplayStatics.OpenLevel` "02_Obstacles")))))

(fn `UserConstructionScript`)