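; BP_LevelTrigger is a key-gated level exit that loads a named level when a player holding the key hits its sprite.
; The PickupKey event sets the HasKey flag that the hit check reads.
; Any other valid hit, keyless player or not, sets PlayerMessage to the key text, and a player leaving the sphere collider swaps it to the hide text.
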(event `self.PaperSprite.OnComponentHit`
  (params (HitComponent :type "PrimitiveComponent Object Reference") (OtherActor :type "Actor Object Reference") (OtherComp :type "PrimitiveComponent Object Reference") (NormalImpulse :type "Vector Structure") (Hit :type "HitResult Structure (by ref)"))
  (`/Engine/EditorBlueprintResources/StandardMacros.IsValid` OtherActor
    (:`Is Valid`
      (if (and (`self.ActorHasTag` OtherActor "Player") (`self.HasKey?`))
        (`GameplayStatics.OpenLevel` (`self.Level Name`))
        (else
          (`TextRenderComponent.K2_SetText` (`self.PlayerMessage`) (`self.DisplayKeyText`)))))))

(event `/Game/_Main/Blueprints/Interfaces/I_DoorKey.PickupKey`
  (set `self.HasKey?` true))

(event `self.Sphere Collider.OnComponentEndOverlap`
  (params (OverlappedComponent :type "PrimitiveComponent Object Reference") (OtherActor :type "Actor Object Reference") (OtherComp :type "PrimitiveComponent Object Reference") (OtherBodyIndex :type Integer))
  (`/Engine/EditorBlueprintResources/StandardMacros.IsValid` OverlappedComponent
    (:`Is Valid`
      (if (`self.ActorHasTag` OtherActor "Player")
        (`TextRenderComponent.K2_SetText` (`self.PlayerMessage`) (`self.HideKeyText`))))))

(fn `UserConstructionScript`)